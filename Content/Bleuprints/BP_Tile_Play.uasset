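; BP_Tile_Play is a playable tile that tracks the player character and can host a tent or portrait child actor.
; Construction sets the child from ChildType, while a box overlap updates PawnOn and the tile type.
; Explode gives visible tiles a one-in-five chance, gated by the tent's flag on Tent tiles, to animate a mesh into an explosion that respawns any player standing there.
; StartPlay's random roll leads nowhere.
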(event OnComponentBeginOverlap(Box)
  (params (OverlappedComponent :type Primitive%20Component%20Object%20Reference) (OtherActor :type Actor%20Object%20Reference) (OtherComp :type Primitive%20Component%20Object%20Reference) (OtherBodyIndex :type Integer) (bFromSweep :type Boolean) (SweepResult :type Hit%20Result%20Structure%20%28by%20ref%29))
  (Utilities|Casting|CastToBP_Char OtherActor)
  (Variables|Default|SetbPawnOn true)
  (CallFunction|SetTileType "NewEnumerator0"))

(event OnComponentEndOverlap(Box)
  (params (OverlappedComponent :type Primitive%20Component%20Object%20Reference) (OtherActor :type Actor%20Object%20Reference) (OtherComp :type Primitive%20Component%20Object%20Reference) (OtherBodyIndex :type Integer))
  (Utilities|Casting|CastToBP_Char OtherActor)
  (Variables|Default|SetbPawnOn false))

(event Custom|StartPlay
  (if (not (Variables|Default|GetbPawnOn))
    (switch int (Math|Random|RandomIntegerinRange 0 3))))

(event Custom|Explode
  (if (Rendering|IsVisible (Variables|Default|GetStaticMesh))
    (switch Utilities|FlowControl|Switch|SwitchonTileChildType (Variables|Default|GetChildType)
      (:NewEnumerator0
        (bind _asbp_tent (Utilities|Casting|CastToBP_Tent (Variables|/Script/Engine.ChildActorComponent|GetChildActor (Variables|Default|GetChildActor))))
        (if (not (Variables|/Game/Bleuprints/BP_Tent.BP_Tent_C|GetbTent _asbp_tent))
          (if (== (Math|Random|RandomIntegerinRange 0 4) 0) :!label _label
            (Rendering|SetVisibility (Variables|Default|GetStaticMesh1) true false)
            (bind _newtrack_0 (Timeline|Timeline_0 PlayFromStart)
              (:Update
                (Transformation|SetRelativeLocation (Variables|Default|GetStaticMesh1) (Math|Vector|Lerp(Vector) (Variables|/Script/Engine.SceneComponent|GetRelativeLocation (Variables|Default|GetStaticMesh1)) "0, 0, 0" _newtrack_0) false false))
              (:Finished
                (Rendering|SetVisibility (Variables|Default|GetStaticMesh1) false false)
                (Effects|Components|ParticleSystem|SetTemplate (Variables|Default|GetParticleSystem) "/Game/MobileStarterContent/Particles/P_Explosion.P_Explosion")
                (Audio|SpawnSoundatLocation "/Game/MobileStarterContent/Audio/Explosion02.Explosion02" (Transformation|GetActorLocation) "0, 0, 0" 1.0 1.0 0.0 0 0)
                (if (Variables|Default|GetbPawnOn)
                  (bind _asbp_plater_ctrl (Utilities|Casting|CastToBP_PlaterCtrl (Game|GetPlayerController 0)))
                  (Default|Respawn _asbp_plater_ctrl)))))))
      (:NewEnumerator1
        (goto _label))
      (:NewEnumerator2
        (goto _label)))))

(event EventBeginPlay
  (|CallParentFunction))

(event EventTick
  (params (DeltaSeconds :type Float%20%28single-precision%29))
  (|CallParentFunction DeltaSeconds))

(fn ConstructionScript
  (bind _childactor (Variables|Default|GetChildActor))
  (|CallParentFunction)
  (Variables|Default|SetBoxColls (Utilities|Array|MakeArray (Variables|Default|GetBox1) (Variables|Default|GetBox2) (Variables|Default|GetBox3) (Variables|Default|GetBox4) (Variables|Default|GetBox5) (Variables|Default|GetBox6) (Variables|Default|GetBox7) (Variables|Default|GetBox8)))
  (switch Utilities|FlowControl|Switch|SwitchonTileChildType (Variables|Default|GetChildType)
    (:NewEnumerator0
      (ChildActorComponent|SetChildActorClass _childactor "/Game/Bleuprints/BP_Tent.BP_Tent_C"))
    (:NewEnumerator1
      (ChildActorComponent|SetChildActorClass _childactor "/Game/Bleuprints/BP_Portrait.BP_Portrait_C")
      (bind _asbp_portrait (Utilities|Casting|CastToBP_Portrait (Variables|/Script/Engine.ChildActorComponent|GetChildActor (Variables|Default|GetChildActor))))
      (Default|SetPortraitType _asbp_portrait (Variables|Default|GetPortraitCount)))))
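; BP_Tile_PlayHelp is a tile that shows tutorial help text when the player steps on it, based on its child type.
; Construction spawns a tent or portrait child actor; box overlaps track player presence and trigger the hints, with the tent's shown once.
; Explode gives Portrait and empty tiles a one-in-four chance to animate a mesh into an explosion, reloading the character if standing there.
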(event OnComponentBeginOverlap(Box)
  (params (OverlappedComponent :type Primitive%20Component%20Object%20Reference) (OtherActor :type Actor%20Object%20Reference) (OtherComp :type Primitive%20Component%20Object%20Reference) (OtherBodyIndex :type Integer) (bFromSweep :type Boolean) (SweepResult :type Hit%20Result%20Structure%20%28by%20ref%29))
  (Utilities|Casting|CastToBP_Char OtherActor)
  (Variables|Default|SetbPawnOn true)
  (CallFunction|SetTileType "NewEnumerator0")
  (bind _asbp_plater_ctrl (Utilities|Casting|CastToBP_PlaterCtrl (Game|GetPlayerController 0)))
  (switch Utilities|FlowControl|Switch|SwitchonTileChildType (Variables|Default|GetChildType)
    (:NewEnumerator0
      (Utilities|FlowControl|DoOnce false
        (:Completed
          (Default|Help _asbp_plater_ctrl "Reach tent before the night.  
Sleep to rejuvenate and dream..."))))
    (:NewEnumerator1
      (Default|Help _asbp_plater_ctrl "This is a fragment of a dream"))))

(event OnComponentEndOverlap(Box)
  (params (OverlappedComponent :type Primitive%20Component%20Object%20Reference) (OtherActor :type Actor%20Object%20Reference) (OtherComp :type Primitive%20Component%20Object%20Reference) (OtherBodyIndex :type Integer))
  (Utilities|Casting|CastToBP_Char OtherActor)
  (Variables|Default|SetbPawnOn false))

(event Custom|StartPlay
  (if (not (Variables|Default|GetbPawnOn))
    (switch int (Math|Random|RandomIntegerinRange 0 3))))

(event Custom|Explode
  (switch Utilities|FlowControl|Switch|SwitchonTileChildType (Variables|Default|GetChildType)
    (:NewEnumerator1
      _)
    (:NewEnumerator2
      _))
  (if (== (Math|Random|RandomIntegerinRange 0 3) 0)
    (Rendering|SetVisibility (Variables|Default|GetStaticMesh1) true false)
    (bind _newtrack_0 (Timeline|Timeline_0 PlayFromStart)
      (:Update
        (Transformation|SetRelativeLocation (Variables|Default|GetStaticMesh1) (Math|Vector|Lerp(Vector) (Variables|/Script/Engine.SceneComponent|GetRelativeLocation (Variables|Default|GetStaticMesh1)) "0, 0, 0" _newtrack_0) false false))
      (:Finished
        (Rendering|SetVisibility (Variables|Default|GetStaticMesh1) false false)
        (Effects|Components|ParticleSystem|SetTemplate (Variables|Default|GetParticleSystem) "/Game/MobileStarterContent/Particles/P_Explosion.P_Explosion")
        (if (Variables|Default|GetbPawnOn)
          (bind _asbp_char (Utilities|Casting|CastToBP_Char (Game|Player|GetPlayerPawn 0)))
          (Default|Reload _asbp_char))))))

(event EventBeginPlay
  (|CallParentFunction))

(event EventTick
  (params (DeltaSeconds :type Float%20%28single-precision%29))
  (|CallParentFunction DeltaSeconds))

(fn ConstructionScript
  (bind _childactor (Variables|Default|GetChildActor))
  (|CallParentFunction)
  (Variables|Default|SetBoxColls (Utilities|Array|MakeArray (Variables|Default|GetBox1) (Variables|Default|GetBox2) (Variables|Default|GetBox3) (Variables|Default|GetBox4) (Variables|Default|GetBox5) (Variables|Default|GetBox6) (Variables|Default|GetBox7) (Variables|Default|GetBox8)))
  (switch Utilities|FlowControl|Switch|SwitchonTileChildType (Variables|Default|GetChildType)
    (:NewEnumerator0
      (ChildActorComponent|SetChildActorClass _childactor "/Game/Bleuprints/BP_Tent.BP_Tent_C"))
    (:NewEnumerator1
      (ChildActorComponent|SetChildActorClass _childactor "/Game/Bleuprints/BP_Portrait.BP_Portrait_C")
      (bind _asbp_portrait (Utilities|Casting|CastToBP_Portrait (Variables|/Script/Engine.ChildActorComponent|GetChildActor (Variables|Default|GetChildActor))))
      (Default|SetPortraitType _asbp_portrait (Variables|Default|GetPortraitCount)))))
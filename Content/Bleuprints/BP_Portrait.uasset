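; BP_Portrait is a spinning collectible portrait that the player character picks up by touch.
; SetPortraitType stores the portrait's index and applies one of nine matching materials to the mesh.
; Tick rotates the mesh by a fixed step each frame, independent of delta time.
; On overlap with BP_Char, it hides the mesh, disables box collision and adds its index to the PortraitCount collection in BP_Instance.
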(event OnComponentBeginOverlap(Box)
  (params (OverlappedComponent :type Primitive%20Component%20Object%20Reference) (OtherActor :type Actor%20Object%20Reference) (OtherComp :type Primitive%20Component%20Object%20Reference) (OtherBodyIndex :type Integer) (bFromSweep :type Boolean) (SweepResult :type Hit%20Result%20Structure%20%28by%20ref%29))
  (Utilities|Casting|CastToBP_Char OtherActor)
  (Rendering|SetVisibility (Variables|Default|GetStaticMesh) false false)
  (Collision|SetCollisionEnabled (Variables|Default|GetBox) "NoCollision")
  (bind _asbp_instance (Utilities|Casting|CastToBP_Instance (Game|GetGameInstance)))
  (Utilities|Array|Add (Variables|/Game/Bleuprints/Game/BP_Instance.BP_Instance_C|GetPortraitCount _asbp_instance) (Variables|Default|GetPortraitCount)))

(event EventTick
  (params (DeltaSeconds :type Float%20%28single-precision%29))
  (Transformation|AddRelativeRotation (Variables|Default|GetStaticMesh) "0,1.000000, 0" false false))

(fn ConstructionScript)

(fn SetPortraitType
  (params (Selection :type Integer))
  (bind _staticmesh (Variables|Default|GetStaticMesh))
  (bind _staticmesh_2 (Variables|Default|GetStaticMesh))
  (bind _output_get (Variables|Default|SetPortraitCount Selection))
  (switch int _output_get
    (:0
      (Rendering|Material|SetMaterial _staticmesh 0 "/Game/Textures/P1_1_Mat.P1_1_Mat"))
    (:1
      (Rendering|Material|SetMaterial _staticmesh 0 "/Game/Textures/P2_1_Mat.P2_1_Mat"))
    (:2
      (Rendering|Material|SetMaterial _staticmesh 0 "/Game/Textures/P3_1_Mat.P3_1_Mat"))
    (:3
      (Rendering|Material|SetMaterial _staticmesh 0 "/Game/Textures/P4_1_Mat.P4_1_Mat"))
    (:4
      (Rendering|Material|SetMaterial _staticmesh 0 "/Game/Textures/P5_1_Mat.P5_1_Mat"))
    (:5
      (Rendering|Material|SetMaterial _staticmesh_2 0 "/Game/Textures/P6_1_Mat.P6_1_Mat"))
    (:6
      (Rendering|Material|SetMaterial _staticmesh_2 0 "/Game/Textures/P7_1_Mat.P7_1_Mat"))
    (:7
      (Rendering|Material|SetMaterial _staticmesh_2 0 "/Game/Textures/P8_1_Mat.P8_1_Mat"))
    (:8
      (Rendering|Material|SetMaterial _staticmesh_2 0 "/Game/Textures/P9_1_Mat.P9_1_Mat"))))
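; BP_Tent is a tent actor that hides the player character inside it when it is not night.
; On box overlap by BP_Char, it checks BP_GM's Night flag, swaps to the closed mesh, and calls HideChar with the parent BP_Tile as the save tile.
; Leaving the box always restores the open mesh and unhides the character, with TentOn choosing the mesh from the Tent boolean.
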(event OnComponentBeginOverlap(Box)
  (params (OverlappedComponent :type Primitive%20Component%20Object%20Reference) (OtherActor :type Actor%20Object%20Reference) (OtherComp :type Primitive%20Component%20Object%20Reference) (OtherBodyIndex :type Integer) (bFromSweep :type Boolean) (SweepResult :type Hit%20Result%20Structure%20%28by%20ref%29))
  (bind _asbp_char (Utilities|Casting|CastToBP_Char OtherActor))
  (bind _asbp_gm (Utilities|Casting|CastToBP_GM (Game|GetGameMode)))
  (if (not (Variables|/Game/Bleuprints/Game/BP_GM.BP_GM_C|GetbNight _asbp_gm))
    (Variables|Default|SetbTent false)
    (CallFunction|Tenton)
    (bind _asbp_tile (Utilities|Casting|CastToBP_Tile (Actor|GetParentActor)))
    (Default|HideChar _asbp_char true _asbp_tile)))

(event OnComponentEndOverlap(Box)
  (params (OverlappedComponent :type Primitive%20Component%20Object%20Reference) (OtherActor :type Actor%20Object%20Reference) (OtherComp :type Primitive%20Component%20Object%20Reference) (OtherBodyIndex :type Integer))
  (bind _asbp_char (Utilities|Casting|CastToBP_Char OtherActor))
  (Variables|Default|SetbTent true)
  (CallFunction|Tenton)
  (Default|HideChar _asbp_char false))

(event Custom|TentOn
  (bind _staticmesh (Variables|Default|GetStaticMesh))
  (if (Variables|Default|GetbTent)
    (Components|StaticMesh|SetStaticMesh _staticmesh "/Game/StaticMeshes/TentOpen.TentOpen")
    (else
      (Components|StaticMesh|SetStaticMesh _staticmesh "/Game/StaticMeshes/TentClosefbx.TentClosefbx"))))

(event EventBeginPlay)

(event Collision|EventActorBeginOverlap
  (params (OtherActor :type Actor%20Object%20Reference)))

(event EventTick
  (params (DeltaSeconds :type Float%20%28single-precision%29)))

(fn ConstructionScript)
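; BP_Tile is a grid tile actor that switches between Walked, Can Walk, Not Walk and Off states.
; SetTileType, also run at construction, swaps the top material or hides the mesh to show the state.
; Neighbours come from the first tile overlapping each box collider.
; Activating marks neighbours as walkable, while deactivating resets those without a pawn on them to not walkable.
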(fn ConstructionScript
  (CallFunction|SetTileType (Variables|Default|GetTileType)))

(fn SetTileType
  (params (TileType :type TileState%20Enum :default "NewEnumerator0"))
  (bind _staticmesh (Variables|Default|GetStaticMesh))
  (switch Utilities|FlowControl|Switch|SwitchonTileState TileType
    (:NewEnumerator0
      (Rendering|Material|SetMaterial _staticmesh 1 "/Game/StaticMeshes/Top2.Top2")
      (Variables|Default|SetTileType "NewEnumerator0")
      (Rendering|SetVisibility (Variables|Default|GetStaticMesh) true false))
    (:NewEnumerator1
      (Rendering|Material|SetMaterial _staticmesh 1 "/Game/StaticMeshes/Top1.Top1")
      (Variables|Default|SetTileType "NewEnumerator1")
      (Rendering|SetVisibility (Variables|Default|GetStaticMesh) true false))
    (:NewEnumerator2
      (Rendering|Material|SetMaterial _staticmesh 1 "/Game/StaticMeshes/Top.Top")
      (Variables|Default|SetTileType "NewEnumerator2")
      (Rendering|SetVisibility (Variables|Default|GetStaticMesh) true false))
    (:NewEnumerator3
      (Rendering|SetVisibility (Variables|Default|GetStaticMesh) false false)
      (Variables|Default|SetTileType "NewEnumerator3"))))

(fn GetNeighbours
  (Utilities|Array|Clear (Variables|Default|GetNeighbourTiles))
  (for _array_element (Variables|Default|GetBoxColls)
    (Utilities|IsValid (Utilities|Array|Get(acopy) (Collision|GetOverlappingActors _array_element "BP_Tile_C" :!class /Script/Engine.PrimitiveComponent))
      (:Is%20Valid
        (bind _asbp_tile (Utilities|Casting|CastToBP_Tile (Utilities|Array|Get(acopy) (Collision|GetOverlappingActors _array_element "BP_Tile_C" :!class /Script/Engine.PrimitiveComponent))))
        (Utilities|Array|Add (Variables|Default|GetNeighbourTiles) _asbp_tile))))
  (return))

(fn ActivateNeighbours
  (CallFunction|GetNeighbours)
  (for _array_element (Variables|Default|GetNeighbourTiles)
    (Utilities|IsValid _array_element
      (:Is%20Valid
        (CallFunction|SetTileType _array_element "NewEnumerator1"))))
  (return))

(fn DeactivateNeighbours
  (CallFunction|GetNeighbours)
  (for _array_element (Variables|Default|GetNeighbourTiles)
    (Utilities|IsValid _array_element
      (:Is%20Valid
        (if (not (Variables|BP_Tile_C|GetbPawnOn _array_element))
          (CallFunction|SetTileType _array_element "NewEnumerator2")))))
  (return))
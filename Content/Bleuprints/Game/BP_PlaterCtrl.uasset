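; Player controller for a tile-based game with click-to-move, stamina and rest mechanics, which also creates the HUD.
; Clicking a tile of the required type lerps the pawn there on a timeline, then updates neighbour tiles and drains stamina, with a HUD warning when exhausted.
; Respawn reloads the pawn at half stamina.
; Dream shows a widget that either declares a win at nine portraits or restores full stamina and continues the game.
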(event Custom|Dream
  (bind _returnvalue (UserInterface|CreateWidget "/Game/UI/WB_Dream.WB_Dream_C"))
  (UserInterface|Viewport|AddtoViewport _returnvalue 0)
  (bind _asbp_instance (Utilities|Casting|CastToBP_Instance (Game|GetGameInstance)))
  (if (== (Utilities|Array|Length (Variables|/Game/Bleuprints/Game/BP_Instance.BP_Instance_C|GetPortraitCount _asbp_instance)) 9)
    (Default|Win _returnvalue)
    (else
      (Utilities|FlowControl|Delay 3.0)
      (Widget|RemovefromParent _returnvalue)
      (Variables|Default|SetStamina 1.0)
      (bind _asbp_gm (Utilities|Casting|CastToBP_GM (Game|GetGameMode)))
      (Default|Continue _asbp_gm)
      (Default|CallStaminaUpdate))))

(event Custom|Help
  (params (InText :type Text))
  (Default|Help (Variables|Default|GetHUD) InText))

(event Custom|Respawn
  (bind _previoustile (Variables|Default|GetPreviousTile))
  (Variables|/Game/Bleuprints/BP_Tile.BP_Tile_C|SetTileType _previoustile "NewEnumerator2")
  (Default|DeactivateNeighbours _previoustile)
  (Default|Reload (Variables|Default|GetPlayerPawn))
  (Variables|Default|SetStamina 0.5)
  (Default|CallStaminaUpdate))

(event EventBeginPlay
  (Variables|Default|SetbEnableClickEvents true)
  (Variables|Default|SetbShowMouseCursor true)
  (bind _returnvalue (UserInterface|CreateWidget "/Game/UI/HUD.HUD_C"))
  (UserInterface|Viewport|AddtoViewport _returnvalue 0)
  (Variables|Default|SetHUD _returnvalue))

(event EventPossess
  (params (PossessedPawn :type Pawn%20Object%20Reference))
  (bind _asbp_char (Utilities|Casting|CastToBP_Char PossessedPawn))
  (Variables|Default|SetPlayerPawn _asbp_char))

(event Input|MouseEvents|LeftMouseButton
  (params (Key :type Key%20Structure :default "None"))
  (bind _playerpawn (Variables|Default|GetPlayerPawn))
  (:Pressed
    (if (Variables|Default|GetbCanClick)
      (if (> (Variables|Default|GetStamina) 0.0)
        (Utilities|IsValid (Variables|Default|GetPlayerPawn)
          (:Is%20Valid
            (bind _asbp_tile (Utilities|Casting|CastToBP_Tile (.hitactor (.HitResult (Game|Player|GetHitResultUnderCursorbyChannel "TraceTypeQuery1" true)))))
            (if (Utilities|Enum|Equal(Enum) (Variables|/Game/Bleuprints/BP_Tile.BP_Tile_C|GetTileType _asbp_tile) "NewEnumerator1")
              (Variables|/Game/Bleuprints/Game/BP_Char.BP_Char_C|SetSpeed (Variables|Default|GetPlayerPawn) 1e+02)
              (Variables|Default|SetbCanClick false)
              (bind _newtrack_0 (Timeline|Timeline_0 PlayFromStart)
                (:Update
                  (Utilities|IsValid _asbp_tile
                    (:Is%20Valid
                      (Transformation|SetActorLocation _playerpawn (Math|Vector|Lerp(Vector) (Transformation|GetActorLocation _playerpawn) (Transformation|GetActorLocation _asbp_tile) _newtrack_0) false false))))
                (:Finished
                  (Variables|Default|SetbCanClick true)
                  (Utilities|IsValid (Variables|Default|GetPreviousTile)
                    (:Is%20Valid
                      (Default|DeactivateNeighbours (Variables|Default|GetPreviousTile))
                      (Variables|/Game/Bleuprints/Game/BP_Char.BP_Char_C|SetSpeed _playerpawn 0.0)
                      (Default|ActivateNeighbours _asbp_tile)
                      (Variables|Default|SetPreviousTile _asbp_tile)
                      (bind _output_get (Variables|Default|SetStamina (- (Variables|Default|GetStamina) 0.1)))
                      (Default|CallStaminaUpdate)
                      (if (<= _output_get 0.0)
                        (Utilities|FlowControl|DoOnce false
                          (:Completed
                            (Default|Help (Variables|Default|GetHUD) "You have lost all stamina. Rest and wait for morning to regain half.  
Tent gives full recharge and sweet dreams.")))))))))))))))

(fn ConstructionScript)
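; BP_GM is the game manager Blueprint that runs the day and night flow around BP_Sun.
; BeginPlay caches the sun and hides play-tile meshes; Start begins the sun cycle and a looping timer whose Play event is empty.
; NightTile01 drains stamina, then triggers Dream if the character's Tent is set, otherwise explodes all tiles repeatedly, waits and restores minimum stamina.
; That branch and Continue both restart the sun cycle and end night.
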(event Custom|Start
  (Default|StartSunCycle (Variables|Default|GetSun))
  (Utilities|Time|SetTimerbyEvent (delegate Custom|Play) 1.5 true))

(event Custom|Play)

(event Custom|NightTile01
  (params (Sun :type BP%20Sun%20Object%20Reference))
  (Variables|Default|SetbNight true)
  (bind _asbp_plater_ctrl (Utilities|Casting|CastToBP_PlaterCtrl (Game|GetPlayerController 0)))
  (Variables|/Game/Bleuprints/Game/BP_PlaterCtrl.BP_PlaterCtrl_C|SetStamina _asbp_plater_ctrl 0.0)
  (Default|CallStaminaUpdate _asbp_plater_ctrl)
  (bind _asbp_char (Utilities|Casting|CastToBP_Char (Game|Player|GetPlayerPawn 0)))
  (if (Variables|/Game/Bleuprints/Game/BP_Char.BP_Char_C|GetbTent _asbp_char)
    (bind _asbp_plater_ctrl_2 (Utilities|Casting|CastToBP_PlaterCtrl (Game|GetPlayerController 0)))
    (Default|Dream _asbp_plater_ctrl_2)
    (else
      (for _index (range 0 4)
        (bind _outactors (Actor|GetAllActorsOfClass "/Game/Bleuprints/BP_Tile_Play.BP_Tile_Play_C"))
        (for _array_element _outactors
          (Default|Explode _array_element)))
      (Utilities|FlowControl|Delay 4.0)
      (bind _asbp_plater_ctrl_3 (Utilities|Casting|CastToBP_PlaterCtrl (Game|GetPlayerController 0)))
      (if (< (Variables|/Game/Bleuprints/Game/BP_PlaterCtrl.BP_PlaterCtrl_C|GetStamina _asbp_plater_ctrl_3) 0.5)
        (Variables|/Game/Bleuprints/Game/BP_PlaterCtrl.BP_PlaterCtrl_C|SetStamina _asbp_plater_ctrl_3 0.5)
        (Default|CallStaminaUpdate _asbp_plater_ctrl_3))
      (Default|StartSunCycle Sun)
      (Variables|Default|SetbNight false))))

(event Custom|Continue
  (Default|StartSunCycle (stale Custom|NightTile01 Sun))
  (Variables|Default|SetbNight false))

(event EventBeginPlay
  (bind _returnvalue (Actor|GetActorOfClass "/Game/Bleuprints/Game/Actors/BP_Sun.BP_Sun_C"))
  (Variables|Default|SetSun _returnvalue)
  (bind _outactors (Actor|GetAllActorsOfClass "/Game/Bleuprints/BP_Tile_Play.BP_Tile_Play_C"))
  (for _array_element _outactors
    (Rendering|SetVisibility (Variables|/Game/Bleuprints/BP_Tile.BP_Tile_C|GetStaticMesh _array_element) false false)))

(fn ConstructionScript)
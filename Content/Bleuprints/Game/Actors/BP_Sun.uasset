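; BP_Sun is an actor that drives a day's sun arc by rotating its directional light.
; It saves the light's starting rotation on BeginPlay, and StartSunCycle restores it through Morning, then starts a looping timer.
; Each tick of that timer steps the pitch until it rises above a horizon threshold, then pauses the timer and calls NightTile01 on the BP_GM game mode.
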(event Custom|StartSunCycle
  (CallFunction|Morning)
  (bind _returnvalue (Utilities|Time|SetTimerbyEvent (delegate Custom|MoveSun) 0.5 true))
  (Variables|Default|SetSunTimer _returnvalue))

(event Custom|MoveSun
  (Transformation|AddWorldRotation (Variables|Default|GetDirectionalLight) (Math|Rotator|MakeRotator 0.0 -1e+01 0.0) false false)
  (if (> (.pitch (Transformation|GetWorldRotation (Variables|Default|GetDirectionalLight))) -1e+01)
    (Utilities|Time|PauseTimerbyHandle (Variables|Default|GetSunTimer))
    (bind _asbp_gm (Utilities|Casting|CastToBP_GM (Game|GetGameMode)))
    (Default|NightTile01 _asbp_gm self)))

(event EventBeginPlay
  (Variables|Default|SetSunDirection (Variables|/Script/Engine.SceneComponent|GetRelativeRotation (Variables|Default|GetDirectionalLight))))

(fn ConstructionScript)

(fn Morning
  (Transformation|SetRelativeRotation (Variables|Default|GetDirectionalLight) (Variables|Default|GetSunDirection) false false))
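; BP_Char is the player character for a tile-based game, with hiding and a saved-tile respawn.
; On begin play it reveals its mesh after a delay, registers with BP_PlaterCtrl as pawn and view target, then activates neighbours of the overlapped BP_Tile.
; HideChar toggles mesh visibility by the Tent flag and stores a save tile when hiding.
; Reload teleports the character to that tile and reactivates its neighbours.
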(event Custom|HideChar
  (params (bTent :type Boolean) (SaveTile :type BP%20Tile%20Object%20Reference))
  (bind _skeletalmesh (Variables|Default|GetSkeletalMesh))
  (bind _output_get (Variables|Default|SetbTent bTent))
  (if _output_get
    (Rendering|SetVisibility _skeletalmesh false false)
    (Variables|Default|SetSaveTile SaveTile)
    (else
      (Rendering|SetVisibility _skeletalmesh true false))))

(event Custom|Reload
  (Transformation|SetActorLocation (Transformation|GetActorLocation (Variables|Default|GetSaveTile)) false false)
  (bind _asbp_plater_ctrl (Utilities|Casting|CastToBP_PlaterCtrl (Game|GetPlayerController 0)))
  (bind _output_get (Variables|/Game/Bleuprints/Game/BP_PlaterCtrl.BP_PlaterCtrl_C|SetPreviousTile _asbp_plater_ctrl (Variables|Default|GetSaveTile)))
  (Default|ActivateNeighbours _output_get))

(event EventBeginPlay
  (bind _returnvalue (Game|GetPlayerController 0))
  (bind _self self)
  (Rendering|SetVisibility (Variables|Default|GetSkeletalMesh) false false)
  (Utilities|FlowControl|Delay 2.2)
  (Rendering|SetVisibility (Variables|Default|GetSkeletalMesh) true false)
  (bind _asbp_plater_ctrl (Utilities|Casting|CastToBP_PlaterCtrl _returnvalue))
  (Variables|/Game/Bleuprints/Game/BP_PlaterCtrl.BP_PlaterCtrl_C|SetPlayerPawn _asbp_plater_ctrl _self)
  (Game|Player|SetViewTargetwithBlend _returnvalue _self 0.0 "VTBlend_Linear" 0.0 false)
  (bind _asbp_tile (Utilities|Casting|CastToBP_Tile (Utilities|Array|Get(acopy) (Collision|GetOverlappingActors (Variables|Default|GetCapsule) "/Game/Bleuprints/BP_Tile.BP_Tile_C" :!class /Script/Engine.PrimitiveComponent))))
  (bind _asbp_plater_ctrl_2 (Utilities|Casting|CastToBP_PlaterCtrl (Game|GetPlayerController 0)))
  (Variables|/Game/Bleuprints/Game/BP_PlaterCtrl.BP_PlaterCtrl_C|SetPreviousTile _asbp_plater_ctrl_2 _asbp_tile)
  (Default|SetTileType _asbp_tile "NewEnumerator0")
  (Default|ActivateNeighbours _asbp_tile))

(fn ConstructionScript)